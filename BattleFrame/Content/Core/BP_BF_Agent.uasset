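; BP_BF_Agent is an agent Blueprint that lays out event hooks for appear, trace, move, attack, hit and death, with no gameplay logic of its own.
; Trace, move, attack and death switch on the incoming data's state, but every branch is empty.
; BeginPlay, Tick and construction only call the parent, and debug prints naming the events are left disconnected.
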(event EventBeginPlay
  (|CallParentFunction))

(event EventOnAppear
  (params (Data :type Appear%20Data%20Structure%20%28by%20ref%29))
  ;[1 1 1] Agent Events
)

(event EventTick
  (params (DeltaSeconds :type Float%20%28single-precision%29))
  (|CallParentFunction DeltaSeconds))

(event EventOnTrace
  (params (Data :type Trace%20Data%20Structure%20%28by%20ref%29))
  ;[1 1 1] Agent Events
  (switch Utilities|FlowControl|Switch|SwitchonETraceEventState (.state Data)))

(event EventOnMove
  (params (Data :type Move%20Data%20Structure%20%28by%20ref%29))
  ;[1 1 1] Agent Events
  (switch Utilities|FlowControl|Switch|SwitchonEMoveEventState (.state Data)))

(event EventOnHit
  (params (Data :type Hit%20Data%20Structure%20%28by%20ref%29))
  ;[1 1 1] Agent Events
)

(event EventOnDeath
  (params (Data :type Death%20Data%20Structure%20%28by%20ref%29))
  ;[1 1 1] Agent Events
  (switch Utilities|FlowControl|Switch|SwitchonEDeathEventState (.state Data)))

(event EventOnAttack
  (params (Data :type Attack%20Data%20Structure%20%28by%20ref%29))
  ;[1 1 1] Agent Events
  (switch Utilities|FlowControl|Switch|SwitchonEAttackEventState (.state Data)))

(fn ConstructionScript
  (|CallParentFunction))